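; HitCheck_BP is an animation notify that performs a hit check at the moment it fires in an animation.
; It sweeps a sphere along offsets rotated to the mesh, filtered by object types and ignoring the owner, with debug drawing enabled.
; A hit applies fixed damage to the single traced actor, then calls OnHitSuccess on the owner if it is an MHPlayer_BP.
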(fn `Received_Notify`
  (params (MeshComp :type "SkeletalMeshComponent Object Reference") (Animation :type "AnimSequenceBase Object Reference"))
  (returns (ReturnValue :type Boolean))
  (bind _returnvalue (`SceneComponent.K2_GetComponentRotation` MeshComp))
  (bind _returnvalue_2 (`ActorComponent.GetOwner` MeshComp))
  (bind _returnvalue_3 (+ (`SceneComponent.K2_GetComponentLocation` MeshComp) (`KismetMathLibrary.GreaterGreater_VectorRotator` (`self.StartOffset`) _returnvalue)))
  (bind (_outhit _returnvalue_4) (`KismetSystemLibrary.SphereTraceSingleForObjects` _returnvalue_3 (+ _returnvalue_3 (`KismetMathLibrary.GreaterGreater_VectorRotator` (`self.EndOffset`) _returnvalue)) (`self.Radius`) (`self.Object Types`) false (`|MakeArray` (`ActorComponent.GetOwner` MeshComp)) "ForDuration"))
  (if _returnvalue_4
    (`|ExecutionSequence`
      (:`then_0`
        (`GameplayStatics.ApplyDamage` (`.HitActor` (`GameplayStatics.BreakHitResult` _outhit)) 50.0))
      (:`then_1`
        (`/Engine/EditorBlueprintResources/StandardMacros.IsValid` _returnvalue_2
          (:`Is Valid`
            (bind _asmhplayer_bp (cast `/Game/1_ProjectMH/Blueprints/Character/MHPlayer_BP` _returnvalue_2))
            (`/Game/1_ProjectMH/Blueprints/Character/MHPlayer_BP.OnHitSuccess` _asmhplayer_bp)
            (return false)))))))