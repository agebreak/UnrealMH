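; MHMob is a mob character Blueprint that takes damage and reacts with dragon hit and death montages.
; While HP is above zero, AnyDamage plays the hit montage, subtracts truncated damage and updates IsDead.
; At zero or below it plays the death montage, then refills HP on completion without clearing IsDead.
; A separate OnDead function destroys the actor but is not called within this Blueprint.
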(event `self.ReceiveTick`
  (params (DeltaSeconds :type "Float (single-precision)")))

(event `self.ReceiveAnyDamage`
  (params (Damage :type "Float (single-precision)") (DamageType :type "DamageType Object Reference") (InstigatedBy :type "Controller Object Reference") (DamageCauser :type "Actor Object Reference"))
  (if (> (`self.HP`) 0)
    (`|ExecutionSequence`
      (:`then_0`
        (`|PlayMontage` (`self.Mesh`) "/Game/1_ProjectMH/Animation/Montage/Dragon_Hit.Dragon_Hit"))
      (:`then_1`
        (bind _output_get (set `self.HP` (- (`self.HP`) (`KismetMathLibrary.FTrunc` Damage))))
        (bind _output_get_2 (set `self.IsDead` (<= _output_get 0)))
        (if _output_get_2
          (`|PlayMontage` (`self.Mesh`) "/Game/1_ProjectMH/Animation/Montage/Dragon_Death.Dragon_Death"
            (:`OnCompleted`
              (set `self.HP` 100))))))))

(fn `OnDead`
  (`self.K2_DestroyActor`))

(fn `UserConstructionScript`)