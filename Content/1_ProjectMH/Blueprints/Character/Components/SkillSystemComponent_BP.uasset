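; Skill system component for the MHPlayer_BP character that plays its attack montages.
; It caches the owning player on BeginPlay.
; OnInputAttack plays the Attack1 montage unless it is already active.
; OnHitSuccess switches to the Attack_Finish montage unless that is already the current montage, forming a hit-triggered follow-up.
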(event `self.ReceiveBeginPlay`
  (bind _asmhplayer_bp (cast `/Game/1_ProjectMH/Blueprints/Character/MHPlayer_BP` (`self.GetOwner`)))
  (set `self.Player` _asmhplayer_bp))

(fn `On Hit Success`
  (bind _player (`self.Player`))
  (if (!= (`Character.GetCurrentMontage` _player) "/Game/1_ProjectMH/Animation/Montage/Attack_Finish.Attack_Finish")
    (`Character.PlayAnimMontage` _player "/Game/1_ProjectMH/Animation/Montage/Attack_Finish.Attack_Finish" 1.0 "None")))

(fn `OnInputAttack`
  (bind _player (`self.Player`))
  (if (not (`AnimInstance.Montage_IsActive` (`SkeletalMeshComponent.GetAnimInstance` (`Character.Mesh` _player)) "/Game/1_ProjectMH/Animation/Montage/Attack1.Attack1"))
    (`Character.PlayAnimMontage` _player "/Game/1_ProjectMH/Animation/Montage/Attack1.Attack1" 1.0 "None")))